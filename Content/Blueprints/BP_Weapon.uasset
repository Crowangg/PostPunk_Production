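; BP_Weapon is a weapon pickup that initializes its ammunition and capacity and can be attached to the player.
; Entering its collision sphere starts a looping timer that traces from the character's camera, updating interaction status for BPI_Interaction actors and passing the weapon's name.
; Leaving the sphere resets that status, and the timer clears itself on its next tick.
; Interact snaps the weapon to the body mesh's WeaponGrip socket and sets WeaponStatus.
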(event OnComponentBeginOverlap(SphereCollision)
  (params (OverlappedComponent :type Primitive%20Component%20Object%20Reference) (OtherActor :type Actor%20Object%20Reference) (OtherComp :type Primitive%20Component%20Object%20Reference) (OtherBodyIndex :type Integer) (bFromSweep :type Boolean) (SweepResult :type Hit%20Result%20Structure%20%28by%20ref%29))
  (bind _asbp_character (Utilities|Casting|CastToBP_Character OtherActor))
  (Variables|Default|SetTriggerStatus true)
  (bind _returnvalue (Utilities|Time|SetTimerbyEvent (delegate Custom|CustomEvent_0) 0.1 true)))

(event OnComponentEndOverlap(SphereCollision)
  (params (OverlappedComponent :type Primitive%20Component%20Object%20Reference) (OtherActor :type Actor%20Object%20Reference) (OtherComp :type Primitive%20Component%20Object%20Reference) (OtherBodyIndex :type Integer))
  (bind _output_get (Variables|Default|SetTriggerStatus false))
  (Variables|/Game/Blueprints/BP_Character.BP_Character_C|SetInteractionStatus (stale OnComponentBeginOverlap(SphereCollision) _asbp_character) false))

(event Custom|CustomEvent_0
  (bind _outhit (Collision|LineTraceByChannel (Transformation|GetWorldLocation (Variables|/Game/Blueprints/BP_Character.BP_Character_C|GetCamera (stale OnComponentBeginOverlap(SphereCollision) _asbp_character))) (+ (Transformation|GetWorldLocation (Variables|/Game/Blueprints/BP_Character.BP_Character_C|GetCamera (stale OnComponentBeginOverlap(SphereCollision) _asbp_character))) (* (Math|Vector|GetForwardVector (Variables|/Game/Blueprints/BP_Character.BP_Character_C|GetCamera (stale OnComponentBeginOverlap(SphereCollision) _asbp_character))) 1.5e+02)) "TraceTypeQuery1" false 0 "ForDuration" false))
  (Variables|/Game/Blueprints/BP_Character.BP_Character_C|SetInteractionStatus (stale OnComponentBeginOverlap(SphereCollision) _asbp_character) (Utilities|DoesObjectImplementInterface (.HitActor (Collision|BreakHitResult _outhit)) "/Game/Blueprints/Interfaces/BPI_Interaction.BPI_Interaction_C"))
  (Variables|/Game/Blueprints/BP_Character.BP_Character_C|SetInteractionActorName (stale OnComponentBeginOverlap(SphereCollision) _asbp_character) (Variables|Default|GetName))
  (if (not (stale OnComponentEndOverlap(SphereCollision) _output_get))
    (Utilities|Time|ClearandInvalidateTimerbyHandle (stale OnComponentBeginOverlap(SphereCollision) _returnvalue))))

(event EventBeginPlay
  (Variables|Default|SetCurrentAmmunition (Variables|Default|GetMaxAmmunition))
  (Variables|Default|SetCurrentCapacity (Variables|Default|GetMaxCapacity))
  (Variables|Default|SetWeaponStatus false))

(fn ConstructionScript)

(fn Interact
  (bind _asbp_character (Utilities|Casting|CastToBP_Character (Game|GetPlayerCharacter 0)))
  (Transformation|AttachComponentToComponent (Variables|/Game/Blueprints/BP_Character.BP_Character_C|GetBodyMesh _asbp_character) "WeaponGrip" "SnapToTarget" "SnapToTarget" "KeepRelative" true)
  (Variables|Default|SetWeaponStatus true)
  (return true))