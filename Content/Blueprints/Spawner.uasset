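; Spawner actor that periodically spawns a configurable class at its Arrow component's location until a set count is reached.
; Tick calls a custom Spawner event, which spawns only while StopSpawn is false and Mob is invalid.
; StopSpawn gates re-entry during the Delay, then stays set once Spawned equals CountOfSpawn.
; The spawned actor is never assigned to Mob in this graph.
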(event Custom|Spawner
  (if (not (Variables|Default|GetStopSpawn))
    (Utilities|IsValid (Variables|Default|GetMob)
      (:Is%20Not%20Valid
        (Variables|Default|SetStopSpawn true)
        (Game|SpawnActorfromClass (Variables|Default|GetObjectToSpawn) (Math|Transform|MakeTransform (Transformation|GetWorldLocation (Variables|Default|GetArrow))) "Undefined" 0 0)
        (bind _result (Math|Integer|IncrementInt (Variables|Default|GetSpawned))
          (:%20%20
            (Variables|Default|SetSpawned _result)
            (Variables|Default|SetNewVar_0 0)
            (Utilities|FlowControl|Delay (Variables|Default|GetTime))
            (Variables|Default|SetStopSpawn (== (Variables|Default|GetCountOfSpawn) (Variables|Default|GetSpawned)))))))))

(event EventTick
  (params (DeltaSeconds :type Float%20%28single-precision%29))
  (CallFunction|Spawner))

(fn ConstructionScript)