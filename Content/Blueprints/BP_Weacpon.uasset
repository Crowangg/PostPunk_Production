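; BP_Weacpon is a weapon pickup that destroys itself when the first-person character uses Action within its sphere.
; Sphere overlap creates a pick-weapon prompt, or rebuilds the health and stamina bars if that widget already exists, and sets Pick.
; Tick polls Pick and the character's Action flag to call PickGun, which only destroys the actor.
; End overlap clears all widgets, recreates the HUD bars and resets Pick.
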(event OnComponentBeginOverlap(Sphere)
  (params (OverlappedComponent :type Primitive%20Component%20Object%20Reference) (OtherActor :type Actor%20Object%20Reference) (OtherComp :type Primitive%20Component%20Object%20Reference) (OtherBodyIndex :type Integer) (bFromSweep :type Boolean) (SweepResult :type Hit%20Result%20Structure%20%28by%20ref%29))
  (bind _returnvalue (Game|GetPlayerController 0))
  (bind _asfirst_person_character (Utilities|Casting|CastToFirstPersonCharacter OtherActor))
  (if (Utilities|IsValid (Variables|Default|GetWidget))
    (Viewport|RemoveAllWidgets)
    (bind _returnvalue_2 (UserInterface|CreateWidget "/Game/Blueprints/BP_Health_bar.BP_Health_bar_C" _returnvalue))
    (bind _returnvalue_3 (UserInterface|CreateWidget "/Game/Blueprints/BP_Stamina_bar.BP_Stamina_bar_C" _returnvalue))
    (UserInterface|Viewport|AddtoViewport _returnvalue_2 0)
    (else
      (bind _returnvalue_4 (UserInterface|CreateWidget "/Game/Blueprints/BP_PickWeapon.BP_PickWeapon_C"))
      (UserInterface|Viewport|AddtoViewport _returnvalue_4 0)
      (Variables|Default|SetWidget _returnvalue_4)))
  (Variables|Default|SetPick true))

(event OnComponentEndOverlap(Sphere)
  (params (OverlappedComponent :type Primitive%20Component%20Object%20Reference) (OtherActor :type Actor%20Object%20Reference) (OtherComp :type Primitive%20Component%20Object%20Reference) (OtherBodyIndex :type Integer))
  (bind _returnvalue (Game|GetPlayerController 0))
  (Viewport|RemoveAllWidgets)
  (bind _returnvalue_2 (UserInterface|CreateWidget "/Game/Blueprints/BP_Health_bar.BP_Health_bar_C" _returnvalue))
  (bind _returnvalue_3 (UserInterface|CreateWidget "/Game/Blueprints/BP_Stamina_bar.BP_Stamina_bar_C" _returnvalue))
  (UserInterface|Viewport|AddtoViewport _returnvalue_2 0)
  (Variables|Default|SetPick false))

(event EventTick
  (params (DeltaSeconds :type Float%20%28single-precision%29))
  (bind _pick (Variables|Default|GetPick))
  (if _pick
    (if (and _pick (Variables|/Game/Blueprints/FirstPersonCharacter.FirstPersonCharacter_C|GetAction (stale OnComponentBeginOverlap(Sphere) _asfirst_person_character)))
      (CallFunction|PickGun))))

(fn ConstructionScript)

(fn PickGun
  (Actor|DestroyActor self))