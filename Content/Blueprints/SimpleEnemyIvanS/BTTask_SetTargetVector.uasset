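; Behavior tree task that picks the next patrol-style destination for an AI_ENEMY pawn from its AI_Controller_Enemy's TargetVectors list.
; It increments the ToMove blackboard index, wrapping to zero at the end of the array, and finishes successfully.
; A second sequence branch, placed after the finish call, writes a random reachable point near the newly indexed vector to the TargetLocation blackboard key.
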(event EventReceiveExecuteAI
  (params (OwnerController :type AI%20Controller%20Object%20Reference) (ControlledPawn :type Pawn%20Object%20Reference))
  (bind _tomove (Variables|Default|GetToMove))
  (bind _returnvalue (Class|BTFunctionLibrary|GetBlackboardValueasInt _tomove))
  (Utilities|FlowControl|Sequence
    (:then_0
      (bind _asai_controller_enemy (Utilities|Casting|CastToAI_Controller_Enemy OwnerController))
      (if (< _returnvalue (- (Utilities|Array|Length (Variables|/Game/Blueprints/SimpleEnemyIvanS/AI_Controller_Enemy.AI_Controller_Enemy_C|GetTargetVectors _asai_controller_enemy)) 1))
        (Class|BTFunctionLibrary|SetBlackboardValueasInt _tomove (+ _returnvalue 1))
        (else
          (Class|BTFunctionLibrary|SetBlackboardValueasInt _tomove)))
      (AI|BehaviorTree|FinishExecute true))
    (:then_1
      (bind _asai_enemy (Utilities|Casting|CastToAI_ENEMY ControlledPawn))
      (AI|Components|Blackboard|SetValueasVector (AI|GetBlackboard _asai_enemy) (Utilities|Name|MakeLiteralName "TargetLocation") (.RandomLocation (AI|Navigation|GetRandomReachablePointinRadius (Utilities|Array|Get(acopy) (Variables|/Game/Blueprints/SimpleEnemyIvanS/AI_Controller_Enemy.AI_Controller_Enemy_C|GetTargetVectors _asai_controller_enemy) (Class|BTFunctionLibrary|GetBlackboardValueasInt (Variables|Default|GetToMove))) 1e+02 0 0))))))