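; Behavior tree task that sets the next move destination for an enemy AI.
; It reads an index from the blackboard, looks up that entry in the enemy controller's TargetVectors, and writes a random reachable navmesh point near it to the ToMove key, then finishes successfully.
; A second sequence branch casts the pawn to AI_ENEMY and re-enters the same logic.
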(event EventReceiveExecuteAI
  (params (OwnerController :type AI%20Controller%20Object%20Reference) (ControlledPawn :type Pawn%20Object%20Reference))
  (Utilities|FlowControl|Sequence
    (:then_0
      (bind _asai_controller_enemy (Utilities|Casting|CastToAI_Controller_Enemy OwnerController)))
    (:then_1
      (Utilities|Casting|CastToAI_ENEMY ControlledPawn)))
  (AI|BehaviorTree|SetBlackboardValueasVector (Variables|Default|GetToMove) (.RandomLocation (AI|Navigation|GetRandomReachablePointinRadius (Utilities|Array|Get(acopy) (Variables|/Game/Blueprints/SimpleEnemyIvanS/AI_Controller_Enemy.AI_Controller_Enemy_C|GetTargetVectors _asai_controller_enemy) (Class|BTFunctionLibrary|GetBlackboardValueasInt (Variables|Default|GetIntIndexTargetVector))) 1e+02 0 "/Script/AIModule.NavFilter_AIControllerDefault")))
  (AI|BehaviorTree|FinishExecute true))