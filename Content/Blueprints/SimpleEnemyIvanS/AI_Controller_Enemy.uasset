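; AI controller for a simple enemy that runs its behavior tree and reacts to player characters it perceives.
; On BeginPlay it seeds the blackboard's TargetLocation with the pawn's position and offsets the pawn's target vectors into world space.
; Perception updates store a character as Enemy, or clear an existing one and move toward it when beyond range.
; Tick only casts the pawn; line-trace and health/distance checks are disconnected.
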(event OnPerceptionUpdated(AIPerception)
  (params (UpdatedActors :type Array%20of%20Actor%20Object%20References))
  (bind _returnvalue (AI|GetBlackboard 0))
  (bind _returnvalue_2 (Utilities|Name|MakeLiteralName "Enemy"))
  (bind _returnvalue_3 (AI|Components|Blackboard|GetValueasObject _returnvalue _returnvalue_2))
  (Utilities|IsValid _returnvalue_3
    (:Is%20Valid
      (Utilities|FlowControl|Sequence
        (:then_0
          (bind _asbp_character (Utilities|Casting|CastToBP_Character _returnvalue_3)
            (:then
              (Utilities|FlowControl|Sequence
                (:then_0
                  (AI|Components|Blackboard|ClearValue _returnvalue _returnvalue_2 :!label _label))
                (:then_1
                  (if (> (Transformation|GetDistanceTo self _asbp_character) 6e+02)
                    (AI|AIMoveTo (Pawn|GetControlledPawn) "0, 0, 0" _asbp_character 6e+02 false
                      (:then
                        (goto _label))
                      (:OnSuccess
                        (goto _label))
                      (:OnFail
                        (goto _label)))))))
            (:CastFailed
              (goto _label))))))
    (:Is%20Not%20Valid
      (bind _array_element (Utilities|Array|ForEachLoopwithBreak UpdatedActors :!label _label_2)
        (:LoopBody
          (bind _asbp_character_2 (Utilities|Casting|CastToBP_Character _array_element))
          (AI|Components|Blackboard|SetValueasObject _returnvalue _returnvalue_2 _asbp_character_2)
          (goto _label_2 Break))))))

(event EventBeginPlay
  (bind _targetvectors (Variables|Default|GetTargetVectors))
  (AI|RunBehaviorTree "/Game/Blueprints/SimpleEnemyIvanS/AI_Enemy_Tree.AI_Enemy_Tree")
  (bind _asai_enemy (Utilities|Casting|CastToAI_ENEMY (Pawn|GetControlledPawn)))
  (AI|Components|Blackboard|SetValueasVector (AI|GetBlackboard 0) (Utilities|Name|MakeLiteralName "TargetLocation") (Transformation|GetWorldLocation (Variables|/Script/Engine.Character|GetCapsuleComponent _asai_enemy)))
  (for _array_element (Variables|/Game/Blueprints/SimpleEnemyIvanS/AI_ENEMY.AI_ENEMY_C|GetTargetsVectors _asai_enemy)
    (Utilities|Array|Add _targetvectors (Math|Vector|MakeVector (+ (.x _array_element) (.x (Transformation|GetWorldLocation (Variables|/Script/Engine.Character|GetCapsuleComponent _asai_enemy)))) (+ (.y _array_element) (.y (Transformation|GetWorldLocation (Variables|/Script/Engine.Character|GetCapsuleComponent _asai_enemy)))) (+ (.z _array_element) (.z (Transformation|GetWorldLocation (Variables|/Script/Engine.Character|GetCapsuleComponent _asai_enemy))))))
    (Utilities|Array|RemoveItem :TargetArray _targetvectors))
  (Utilities|Array|RemoveItem :TargetArray _targetvectors))

(event EventTick
  (params (DeltaSeconds :type Float%20%28single-precision%29))
  (bind _asai_enemy (Utilities|Casting|CastToAI_ENEMY (Pawn|GetControlledPawn))))

(fn ConstructionScript)